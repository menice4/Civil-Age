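; Master building Blueprint for the hex-grid RTS, handling display mesh, resource cost and bulldozing.
; The construction script sets the mesh, scales the click Box to its bounds and fills the Cost map from CostStruct.
; OpenGate and CloseGate toggle bulldoze mode, with hand cursor and red hover material.
; Clicking then restores overlapped used tiles as HexGrid child actors and destroys the building, with one type also updating gatherer state.
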(event OnBeginCursorOver(Box)
  (params (TouchedComponent :type Primitive%20Component%20Object%20Reference))
  (if (Variables|Default|GetBulldoze_mode)
    (Rendering|Material|SetMaterial (Variables|Default|GetStaticMesh) 0 "/AnimationSharing/AnimSharingRed.AnimSharingRed")))

(event OnEndCursorOver(Box)
  (params (TouchedComponent :type Primitive%20Component%20Object%20Reference))
  (if (Variables|Default|GetBulldoze_mode)
    (Rendering|Material|SetMaterial (Variables|Default|GetStaticMesh) 0 (Variables|Default|GetMaterial))))

(event OnClicked(Box)
  (params (TouchedComponent :type Primitive%20Component%20Object%20Reference) (ButtonPressed :type Key%20Structure))
  (if (Variables|Default|GetBulldoze_mode)
    (if (Utilities|Enum|Equal(Enum) (Variables|Default|GetBuilding_type) "NewEnumerator1")
      (Variables|/Game/Resource/Node_Parent.Node_Parent_C|SetActive (Variables|/Game/RTS_Controler.RTS_Controler_C|GetGatherer (.AsRTS%20Controler (Utilities|Casting|CastToRTS_Controler (Game|GetPlayerController 0)))) true)
      (bind _outactors (Actor|GetAllActorswithInterface "/Game/Resource/Resource_Interface.Resource_Interface_C"))
      (for _array_element _outactors
        (Class|ResourceInterface|RemoveGathere(Message) _array_element (Variables|Default|GetBuilding%20Name))
        (for _array_element_2 (Collision|GetOverlappingActors (Variables|Default|GetBox) "/Game/Hex_Tile_used.Hex_Tile_used_C" :!class /Script/Engine.PrimitiveComponent) :!label _label
          (bind _returnvalue (Actor|GetActorOfClass "/Game/HexGrid_BP.HexGrid_BP_C"))
          (bind _returnvalue_2 (AddComponent|AddChildActorComponent _returnvalue false (Transformation|GetActorTransform _array_element_2)))
          (ChildActorComponent|SetChildActorClass _returnvalue_2 "/Game/Hex_Tile_BP.Hex_Tile_BP_C")
          (Actor|DestroyActor _array_element_2)
          (goto _label))
        (Utilities|FlowControl|Delay 0.01)
        (Actor|DestroyActor))
      (else
        (for _array_element_3 (Collision|GetOverlappingActors (Variables|Default|GetBox) "/Game/Hex_Tile_used.Hex_Tile_used_C" :!class /Script/Engine.PrimitiveComponent) :!label _label_2
          (bind _returnvalue_3 (Actor|GetActorOfClass "/Game/HexGrid_BP.HexGrid_BP_C"))
          (bind _returnvalue_4 (AddComponent|AddChildActorComponent _returnvalue_3 false (Transformation|GetActorTransform _array_element_3)))
          (ChildActorComponent|SetChildActorClass _returnvalue_4 "/Game/Hex_Tile_BP.Hex_Tile_BP_C")
          (Actor|DestroyActor _array_element_3)
          (goto _label_2))
        (Utilities|FlowControl|Delay 0.01)
        (Actor|DestroyActor)))))

(event Custom|Open%20Gate
  (Variables|Default|SetBulldoze_mode true)
  (Variables|/Script/Engine.PlayerController|SetCurrentMouseCursor (Game|GetPlayerController 0) "Hand"))

(event Custom|Close%20Gate
  (Variables|Default|SetBulldoze_mode false)
  (Variables|/Script/Engine.PlayerController|SetCurrentMouseCursor (Game|GetPlayerController 0) "Default"))

(event EventBeginPlay
  (Utilities|FlowControl|Sequence
    (:then_0
      (bind _returnvalue (Actor|GetActorOfClass "/Game/Hex_Tile_used.Hex_Tile_used_C"))
      (Variables|Default|SetHex_tile_used _returnvalue)
      (Variables|Default|SetMaterial (Rendering|Material|GetMaterial (Variables|Default|GetStaticMesh) 0))
      (Variables|Default|SetBuilding%20Name "None"))))

(fn ConstructionScript
  (bind _cost_struct (Variables|Default|GetCost_struct))
  (bind _box (Variables|Default|GetBox))
  (bind _staticmesh (Variables|Default|GetStaticMesh))
  (bind _boxextent (Collision|GetComponentBounds _box))
  (bind _boxextent_2 (Collision|GetComponentBounds _staticmesh))
  (bind _returnvalue (* _boxextent_2 "2.000000,2.000000,2.000000"))
  (bind _returnvalue_2 (* _boxextent "1.000000,1.000000,1.000000"))
  (bind _returnvalue_3 (/ _returnvalue _returnvalue_2))
  (bind _array (Utilities|Array|MakeArray (.x _returnvalue_3) (.y _returnvalue_3) (.z _returnvalue_3)))
  (bind _minvalue (Math|Float|MinOfFloatArray _array))
  (Components|StaticMesh|SetStaticMesh (Variables|Default|GetStaticMesh) (Variables|Default|GetDIsplayMesh))
  (Transformation|SetRelativeScale3D (Variables|Default|GetBox) (Math|Vector|MakeVector _minvalue _minvalue (+ _minvalue (Variables|Default|GetZ%20offset))))
  (for _array_element (Variables|Default|GetResource_Da)
    (Utilities|Map|Add (Variables|Default|GetCost) (Variables|/Game/Resource/Resource_DA.Resource_DA_C|GetName _array_element) 0)
    (Utilities|SetCost (.rock _cost_struct) (.iron _cost_struct) (.copper _cost_struct))))

(fn FindResourceName
  (params (ItemToFind :type Resource%20DA%20Object%20Reference))
  (bind _resource_da (Variables|Default|GetResource_Da))
  (return (Variables|/Game/Resource/Resource_DA.Resource_DA_C|GetName (Utilities|Array|Get(acopy) _resource_da (Utilities|Array|FindItem _resource_da ItemToFind)))))

(fn SetResource
  (params (Value :type Integer%20%28by%20ref%29) (ItemToFind :type Resource%20DA%20Object%20Reference))
  (Utilities|Map|Add (Variables|Default|GetCost) (CallFunction|FindResourceName ItemToFind) Value))

(fn BuildCost
  (return))