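; Base Blueprint, by its name, for resource gatherer buildings that register their output with the game's Resource_Master actor.
; On BeginPlay it finds that actor and adds its ResourceStruct count to the Gathereer map entry for that resource name.
; An older approach using Resource_Interface broadcasts and a looping timer remains disconnected, and Tick is empty.
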(event Custom|Tick)

(event EventBeginPlay
  (bind _resource_struct (Variables|Default|GetResource%20struct))
  (bind _returnvalue (Actor|GetActorOfClass "/Game/Resource/Resource_Master.Resource_Master_C"))
  (Utilities|FlowControl|Sequence
    (:then_0
      (Utilities|Map|Add (Variables|/Game/Resource/Resource_Master.Resource_Master_C|Getgathereer _returnvalue) (.name _resource_struct) (+ (.Value (Utilities|Map|Find (Variables|/Game/Resource/Resource_Master.Resource_Master_C|Getgathereer _returnvalue) (.name _resource_struct))) (.count _resource_struct))))))

(fn ConstructionScript
  (|CallParentFunction))