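; Base gatherer building Blueprint that registers its resource type with the game's Resource_Master.
; On BeginPlay it finds GhostBuilding_BP, waits briefly, and if that actor's Ghost flag is off, sends the ResourcesDa name to Resource_Master through AddGathereMessage.
; The remaining graph logic for interface lookups, timers, resource maps and cost printing is disconnected and never runs.
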(event EventBeginPlay
  (bind _returnvalue (Actor|GetActorOfClass "/Game/Buildings/GhostBuilding_BP.GhostBuilding_BP_C"))
  (Utilities|FlowControl|Delay 0.2)
  (if (not (Variables|/Game/Buildings/GhostBuilding_BP.GhostBuilding_BP_C|GetGhost? _returnvalue))
    (bind _returnvalue_2 (Actor|GetActorOfClass "/Game/Resource/Resource_Master.Resource_Master_C"))
    (Class|ResourceInterface|AddGathere(Message) _returnvalue_2 (Variables|/Game/Resource/Resource_DA.Resource_DA_C|GetName (Variables|Default|GetResources_Da)))))

(fn ConstructionScript
  (|CallParentFunction))