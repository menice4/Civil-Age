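; Placement preview actor that shows a translucent ghost of the selected building in RTS build mode.
; ConstructBuilding briefly spawns the real building to read its mesh, types, proxy and build time, then destroys it and activates the ghost.
; While active, a gated Tick follows the Hex position, swaps material by tile and resource-node compatibility, and sets the controller's NotBlocked flag.
; It rotates in 45-degree steps and exposes a construction struct for placement.
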(event Custom|OnSpawn
  (params (DisplayMesh :type Static%20Mesh%20Object%20Reference) (BuildingClass :type Building%20M%20Aster%20BP%20Class%20Reference) (ConstructionProxy :type Construction%20Proxy%20Bp%20Class%20Reference) (BuildTime :type Float%20%28double-precision%29))
  (if (not (Variables|Default|GetIsActive))
    (Variables|Default|SetBuildingClass BuildingClass)
    (Variables|Default|SetConstructionProxy ConstructionProxy)
    (Variables|Default|SetDisplayMesh DisplayMesh)
    (Variables|Default|SetBuildTime BuildTime)
    (Variables|Default|SetIsActive true)
    (Variables|/Game/RTS_Controler.RTS_Controler_C|SetBuildModeActive (Variables|Default|GetControllerReference%20) true)
    (Components|StaticMesh|SetStaticMesh (Variables|Default|GetGhostBuilding_mesh) (Variables|Default|GetDisplayMesh))
    (Rendering|Material|SetMaterial (Variables|Default|GetGhostBuilding_mesh) 0 "/Game/Materials/Ghost_valid.Ghost_valid")
    (CallFunction|OpenTickGate)))

(event Custom|KillGhost
  (Variables|Default|SetBuildingClass 0)
  (Variables|Default|SetConstructionProxy 0)
  (CallFunction|CloseTickGate)
  (Variables|Default|SetDisplayMesh 0)
  (Variables|Default|SetIsActive false)
  (Variables|/Game/RTS_Controler.RTS_Controler_C|SetBuildModeActive (Variables|Default|GetControllerReference%20) false)
  (Components|StaticMesh|SetStaticMesh (Variables|Default|GetGhostBuilding_mesh) (Variables|Default|GetDisplayMesh)))

(event Custom|OpenTickGate
  (bind _hex (Variables|Default|GetHex))
  (bind _tile_type (Variables|Default|GetTile_type))
  (bind _ghostbuilding_mesh (Variables|Default|GetGhostBuilding_mesh))
  (bind _building_type (Variables|Default|GetBuilding%20Type))
  (Variables|Default|SetGhost? true)
  (Utilities|FlowControl|Gate true) ; enters at Open
)

(event Custom|CloseTickGate
  (bind _hex (Variables|Default|GetHex))
  (bind _tile_type (Variables|Default|GetTile_type))
  (bind _ghostbuilding_mesh (Variables|Default|GetGhostBuilding_mesh))
  (bind _building_type (Variables|Default|GetBuilding%20Type))
  (Variables|Default|SetGhost? false)
  (Utilities|FlowControl|Gate true) ; enters at Close
)

(event Custom|RotateAntiClockwise
  (bind _self self)
  (bind _ghostbuilding_mesh (Variables|Default|GetGhostBuilding_mesh _self))
  (bind _returnvalue (Transformation|GetSocketRotation _ghostbuilding_mesh "None"))
  (if (Variables|Default|GetGhost?)
    (Transformation|SetActorRotation (Math|Rotator|MakeRotator (.roll _returnvalue) (.pitch _returnvalue) (- (.yaw _returnvalue) 45.0)))))

(event Custom|RotateClockwise
  (bind _self self)
  (bind _ghostbuilding_mesh (Variables|Default|GetGhostBuilding_mesh _self))
  (bind _returnvalue (Transformation|GetSocketRotation _ghostbuilding_mesh "None"))
  (if (Variables|Default|GetGhost?)
    (Transformation|SetActorRotation _self (Math|Rotator|MakeRotator (.roll _returnvalue) (.pitch _returnvalue) (+ (.yaw _returnvalue) 45.0)))))

(event EventConstructBuilding
  (params (MainBuilding :type Building%20M%20Aster%20BP%20Class%20Reference) (Transform :type Transform))
  (bind _returnvalue (Game|SpawnActorfromClass MainBuilding (Math|Transform|MakeTransform (Math|Vector|MakeVector 0.0 0.0 75.0) "0, 0, 0" "1.000000,1.000000,1.000000") "AlwaysSpawn" "MultiplyWithRoot" 0 (Variables|Default|GetControllerReference%20) "NewEnumerator1" 0))
  (Utilities|FlowControl|Sequence
    (:then_0
      (bind _output_get (Variables|Default|SetNew%20Transform (Transformation|GetWorldTransform (Variables|/Game/Buildings/BuildingMAster_BP.BuildingMAster_BP_C|GetStaticMesh _returnvalue))))
      (bind _asbuilding_master_bp (Utilities|Casting|CastToBuildingMAster_BPClass MainBuilding))
      (if (Variables|/Game/Buildings/BuildingMAster_BP.BuildingMAster_BP_C|GetGatherer? _returnvalue)
        (Variables|Default|SetgatherType (Variables|/Game/Buildings/BuildingMAster_BP.BuildingMAster_BP_C|GetResourceType _returnvalue)))
      (Variables|Default|SetBuilding%20Type (Variables|/Game/Buildings/BuildingMAster_BP.BuildingMAster_BP_C|GetBuilding_type _returnvalue))
      (CallFunction|KillGhost)
      (Utilities|FlowControl|Delay 0.2)
      (CallFunction|OnSpawn (Variables|/Game/Buildings/BuildingMAster_BP.BuildingMAster_BP_C|GetDIsplayMesh _returnvalue) _asbuilding_master_bp (Variables|/Game/Buildings/BuildingMAster_BP.BuildingMAster_BP_C|GetConstructionProxy _returnvalue) (Variables|/Game/Buildings/BuildingMAster_BP.BuildingMAster_BP_C|GetConstructionTime _returnvalue)))
    (:then_1
      (Utilities|FlowControl|Delay 0.2)
      (Actor|DestroyActor _returnvalue))))

(event EventBeginPlay
  (Utilities|Refence))

(event EventTick
  (params (DeltaSeconds :type Float%20%28single-precision%29))
  (bind _hex (Variables|Default|GetHex))
  (bind _tile_type (Variables|Default|GetTile_type))
  (bind _ghostbuilding_mesh (Variables|Default|GetGhostBuilding_mesh))
  (bind _building_type (Variables|Default|GetBuilding%20Type))
  (Utilities|FlowControl|Gate true
    (:Exit
      (Transformation|SetActorLocation self (Math|Vector|MakeVector (.x _hex) (.y _hex) (+ (.z _hex) 75.0)) false false)
      (Utilities|FlowControl|Sequence
        (:then_0
          (if (Utilities|Enum|Equal(Enum) _building_type _tile_type)
            (if (Utilities|Enum|Equal(Enum) (Variables|Default|GetgatherType) (Variables|Default|GetNode_type))
              (Rendering|Material|SetMaterial _ghostbuilding_mesh 0 (Variables|Default|Getmaterial))
              (Utilities|FlowControl|DoOnce false :!label _label
                (:Completed
                  (bind _asrts_controler (Utilities|Casting|CastToRTS_Controler (Game|GetPlayerController 0)))
                  (Variables|/Game/RTS_Controler.RTS_Controler_C|SetNotBlocked _asrts_controler true)))
              (else
                (Utilities|FlowControl|Sequence :!label _label_2
                  (:then_0
                    (if (and (Utilities|Enum|Equal(Enum) _building_type "NewEnumerator0") (Utilities|Enum|NotEqual(Enum) _tile_type "NewEnumerator1"))
                      (Utilities|FlowControl|Sequence
                        (:then_0
                          (Rendering|Material|SetMaterial _ghostbuilding_mesh 0 (Variables|Default|Getmaterial))
                          (Utilities|FlowControl|DoOnce false :!label _label_3
                            (:Completed
                              (bind _asrts_controler_2 (Utilities|Casting|CastToRTS_Controler (Game|GetPlayerController 0)))
                              (Variables|/Game/RTS_Controler.RTS_Controler_C|SetNotBlocked _asrts_controler_2 true))))
                        (:then_1
                          (goto _label_3 Reset)))
                      (else
                        (Rendering|Material|SetMaterial _ghostbuilding_mesh 0 "/Game/Materials/Ghost_invalid.Ghost_invalid")
                        (Utilities|FlowControl|DoOnce false :!label _label_4
                          (:Completed
                            (bind _asrts_controler_3 (Utilities|Casting|CastToRTS_Controler (Game|GetPlayerController 0)))
                            (Variables|/Game/RTS_Controler.RTS_Controler_C|SetNotBlocked _asrts_controler_3 false))))))
                  (:then_1
                    (goto _label Reset)))))
            (else
              (goto _label_2))))
        (:then_1
          (goto _label_4 Reset))))))

(fn ConstructionScript)

(fn SetGridSnapVector
  (bind _cursorworldpostion (Variables|Default|GetCursorWorldPostion))
  (bind _gridsize (Variables|Default|GetGridSize))
  (return (Math|Vector|MakeVector (CallFunction|GridSnap (.x _cursorworldpostion) _gridsize) (CallFunction|GridSnap (.y _cursorworldpostion) _gridsize) (CallFunction|GridSnap (.z _cursorworldpostion) _gridsize))))

(fn SetCursorPositon
  (params (Cursor%20Location :type Vector))
  (Variables|Default|SetCursorWorldPosition Cursor%20Location)
  (return))

(fn GetConstructionStruct
  (return (Utilities|Struct|MakeConstruction_struct (Variables|Default|GetBuildingClass) (Variables|Default|GetConstructionProxy) (Math|Transform|MakeTransform (Transformation|GetActorLocation) (Transformation|GetActorRotation)) (Variables|Default|GetDisplayMesh) (Variables|Default|GetBuildTime))))

(fn GetCost
  (bind _cost (Variables|Default|GetCost))
  (return (Utilities|Struct|MakeCosts (.rock _cost) (.concrete _cost) (.iron _cost) (.copper _cost))))

(fn SetCalendar
  (params (Date :type Array%20of%20Integers))
  (return false))

(fn SetClock
  (params (Time :type Array%20of%20Integers))
  (return false))