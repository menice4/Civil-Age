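; Hex grid actor that lays out tiles and turns the hovered one into a live Hex_Tile_BP actor.
; The construction script builds staggered rows from mesh bounds, scale and offset, as either mesh instances or child tile actors.
; On cursor-over, a DoOnce finds the hit instance, hides it by zero scale and spawns a tile actor carrying its transform and index.
; Returninstance only resets that gate; the instance-restore node is unconnected.
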(event Custom|Return%20instance
  (Utilities|FlowControl|DoOnce false) ; enters at Reset
)

(event Custom|CustomEvent)

(event MouseInput|EventActorBeginCursorOver
  (Utilities|FlowControl|DoOnce false
    (:Completed
      (Variables|Default|SetCurrent%20Instance%20Hit (.HitItem (Collision|BreakHitResult (.HitResult (Game|Player|GetHitResultUnderCursorbyChannel (Game|GetPlayerController 0) "TraceTypeQuery4" true)))))
      (Variables|Default|SetCurrent%20%20Instance%20Transform (.OutInstanceTransform (Components|InstancedStaticMesh|GetInstanceTransform (Variables|Default|GetInstancedStaticMesh) (Variables|Default|GetCurrent%20Instance%20Hit) true)))
      (Components|InstancedStaticMesh|UpdateInstanceTransform (Variables|Default|GetInstancedStaticMesh) (Variables|Default|GetCurrent%20Instance%20Hit) (Math|Transform|MakeTransform (.location (Variables|Default|GetCurrent%20%20Instance%20Transform)) (.rotation (Variables|Default|GetCurrent%20%20Instance%20Transform)) "0.000000,0.000000,0.000000") true true false)
      (bind _output_get (CallFunction|AddTileActor))
      (bind _output_get_2 (Variables|/Game/Hex_Tile_BP.Hex_Tile_BP_C|SetLocation _output_get (Variables|Default|GetCurrent%20%20Instance%20Transform)))
      (Development|PrintString (Utilities|String|ToString(Transform) _output_get_2))
      (bind _output_get_3 (Variables|/Game/Hex_Tile_BP.Hex_Tile_BP_C|SetIndex _output_get (Variables|Default|GetCurrent%20Instance%20Hit)))
      (Development|PrintString (Utilities|String|ToString(Integer) _output_get_3)))))

(event EventTick
  (params (DeltaSeconds :type Float%20%28single-precision%29)))

(event EventBeginPlay
  (bind _returnvalue (Actor|GetActorOfClass "/Game/Buildings/GhostBuilding_BP.GhostBuilding_BP_C"))
  (Variables|Default|SetGhostBuilding _returnvalue))

(fn ConstructionScript
  (bind _scale (Variables|Default|GetScale))
  (bind _returnvalue (Math|Conversions|ToVector(Float) _scale))
  (Components|StaticMesh|SetStaticMesh (Variables|Default|GetInstancedStaticMesh) (Variables|Default|GetTileMesh))
  (Variables|Default|SetRadius (* (.x (.max (StaticMesh|GetBoundingBox (Variables|Default|GetTileMesh)))) (Variables|Default|GetScale)))
  (for _index (range 0 (Variables|Default|GetHeight))
    (for _index_2 (range 0 (- (Variables|Default|GetWidth) 1))
      (if (Variables|Default|GetInstance)
        (Variables|Default|SetX (+ (* _index_2 (Variables|Default|GetRadius) 2.0) (* _index_2 (Variables|Default|GetOffset)) (Variables|Default|GetRowOffset)))
        (Variables|Default|SetY (+ (* _index (Variables|Default|GetOffset)) (* (/ (* (Variables|Default|GetRadius) 2.0) (Math|Float|Sqrt 3.0)) 1.5 _index)))
        (Components|InstancedStaticMesh|AddInstance (Variables|Default|GetInstancedStaticMesh) (Math|Transform|MakeTransform (Math|Vector|MakeVector (+ (* _index_2 (Variables|Default|GetRadius) 2.0) (* _index_2 (Variables|Default|GetOffset)) (Variables|Default|GetRowOffset)) (+ (* _index (Variables|Default|GetOffset)) (* (/ (* (Variables|Default|GetRadius) 2.0) (Math|Float|Sqrt 3.0)) 1.5 _index)) 0.0) "0, 0, 0" _returnvalue) false)
        (else
          (bind _returnvalue_2 (AddComponent|AddChildActorComponent false (Math|Transform|MakeTransform (Math|Vector|MakeVector (+ (* _index_2 (Variables|Default|GetRadius) 2.0) (* _index_2 (Variables|Default|GetOffset)) (Variables|Default|GetRowOffset)) (+ (* _index (Variables|Default|GetOffset)) (* (/ (* (Variables|Default|GetRadius) 2.0) (Math|Float|Sqrt 3.0)) 1.5 _index)) 0.0) "0, 0, 0" _returnvalue)))
          (ChildActorComponent|SetChildActorClass _returnvalue_2 "/Game/Hex_Tile_BP.Hex_Tile_BP_C"))))
    (Utilities|FlowControl|FlipFlop
      (:A
        (Variables|Default|SetRowOffset (* (Variables|Default|GetRadius) -1.0)))
      (:B
        (Variables|Default|SetRowOffset 0.0)))))

(fn AddTileActor
  (bind _returnvalue (Game|SpawnActorfromClass "/Game/Hex_Tile_BP.Hex_Tile_BP_C" (Variables|Default|GetCurrent%20%20Instance%20Transform) "AlwaysSpawn" "MultiplyWithRoot" 0 0))
  (bind _output_get (Variables|Default|SetSwappedActor _returnvalue))
  (Variables|Default|SetActor%20Active true)
  (return _output_get))