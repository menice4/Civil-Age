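; Hex tile actor for an RTS-style grid that shows a top highlight on cursor hover and feeds the building ghost.
; Hover passes the tile's Center socket location and TileType to GhostBuilding_BP, and BeginPlay caches HexGrid_BP.
; Placed resets the material, lowers the mesh and removes the tile from the RTS controller's HexTileRef list.
; Selection, visibility and instanced-mesh swap logic is left disconnected and never runs.
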(event OnEndCursorOver(Tile)
  (params (TouchedComponent :type Primitive%20Component%20Object%20Reference))
  (Development|SetHiddeninGame (Variables|Default|GetHextop) true false))

(event OnBeginCursorOver(Tile)
  (params (TouchedComponent :type Primitive%20Component%20Object%20Reference))
  (Development|SetHiddeninGame (Variables|Default|GetHextop) false false)
  (bind _returnvalue (Actor|GetActorOfClass "/Game/Buildings/GhostBuilding_BP.GhostBuilding_BP_C"))
  (Variables|/Game/Buildings/GhostBuilding_BP.GhostBuilding_BP_C|SetHex _returnvalue (Transformation|GetSocketLocation (Variables|Default|GetTile) "Center"))
  (Variables|/Game/Buildings/GhostBuilding_BP.GhostBuilding_BP_C|SetTile_type _returnvalue (Variables|Default|GetTile%20type)))

(event EventBeginPlay
  (bind _returnvalue (Actor|GetActorOfClass "/Game/HexGrid_BP.HexGrid_BP_C"))
  (Variables|Default|SetHex_grid _returnvalue))

(event Collision|EventActorBeginOverlap
  (params (OtherActor :type Actor%20Object%20Reference)))

(fn ConstructionScript)

(fn Placed
  (bind _tile (Variables|Default|GetTile))
  (bind _returnvalue (Transformation|GetWorldLocation _tile))
  (Rendering|Material|SetMaterial _tile 0 "/Engine/MapTemplates/Materials/BasicAsset01.BasicAsset01")
  (Transformation|SetWorldLocation _tile (Math|Vector|MakeVector (.x _returnvalue) (.y _returnvalue) (- (.z _returnvalue) 7.0)) false false)
  (bind _asrts_controler (Utilities|Casting|CastToRTS_Controler (Game|GetPlayerController 0)))
  (Utilities|Array|RemoveItem (Variables|/Game/RTS_Controler.RTS_Controler_C|GetHex_tile_ref _asrts_controler) self))