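; Construction proxy actor that shows a mesh with a ghost material as a placeholder while something is being built.
; Each tick it advances a clock by delta time and a time unit, which a handler updates for game-speed changes from the game state.
; When work time reaches the configured construction time, it broadcasts completion and destroys itself after a short delay.
; Work time is printed on screen for debugging.
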(event Custom|AjustTime
  (params (TimeUnit :type Float%20%28double-precision%29))
  (Variables|Default|SetTimeUnit TimeUnit))

(event EventBeginPlay
  (bind _output_get (Variables|Default|SetAs%20My%20Game%20State (.AsMy%20Game%20State (Utilities|Casting|CastToMy_gameState (Game|GetGameState)))))
  (EventDispatchers|BindEventtoUpdateGameSpeed _output_get (EventDispatchers|CreateEvent :!event Custom|AjustTime)))

(event Collision|EventActorBeginOverlap
  (params (OtherActor :type Actor%20Object%20Reference)))

(event EventTick
  (params (DeltaSeconds :type Float%20%28single-precision%29))
  (Development|PrintString (Utilities|String|ToString(Float) (Variables|Default|GetWorkTimeSpent)))
  (Variables|Default|SetDelta%20Seconds DeltaSeconds)
  (if (not (Variables|Default|GetConstructionComplete?))
    (CallFunction|DoWork)
    (if (>= (Variables|Default|GetWorkTimeSpent) (Variables|Default|GetConstructTime))
      (Variables|Default|SetConstructionComplete? true)
      (Default|CallConstructionCompleted self)
      (Utilities|FlowControl|Delay 0.2)
      (Actor|DestroyActor))))

(fn ConstructionScript
  (bind _staticmesh (Variables|Default|GetStaticMesh))
  (Components|StaticMesh|SetStaticMesh _staticmesh (Variables|Default|GetDisplayMesh))
  (Rendering|Material|SetMaterial _staticmesh 0 "/Game/Materials/Ghost_Proxy.Ghost_Proxy"))

(fn SetConstructionTime
  (params (BuildTime :type Float%20%28double-precision%29))
  (Variables|Default|SetConstructTime (* BuildTime 6e+01))
  (return))

(fn DoWork
  (bind _output_get (Variables|Default|SetClockwork (.ClockworkOut (CallFunction|SetClockwork (Variables|Default|GetDelta%20Seconds) (Variables|Default|GetTimeUnit) (Variables|Default|GetClockwork)))))
  (bind _output_get_2 (Variables|Default|SetWorkTimeSpent (* _output_get 6e+01)))
  (Development|PrintString (Utilities|String|ToString(Float) _output_get_2))
  (return))