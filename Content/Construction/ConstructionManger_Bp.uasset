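; Construction manager that turns building requests into timed proxy actors and replaces them with the finished buildings.
; QueueConstruction spawns a proxy with the display mesh, binds its completion event, sets its build time and records it in parallel Proxies and Queue arrays.
; On completion, FinishConstruction uses the proxy's index to retrieve its config, removes both entries, spawns the building at the stored transform and destroys the proxy.
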(event Custom|BindConstruction
  (params (Proxy :type Construction%20Proxy%20Bp%20Object%20Reference))
  (EventDispatchers|BindEventtoConstructionCompleted Proxy (EventDispatchers|CreateEvent :!event Custom|ConstructionCompleted)))

(event Custom|ConstructionCompleted
  (params (Proxy :type Construction%20Proxy%20Bp%20Object%20Reference))
  (CallFunction|FinishConstruction Proxy))

(fn ConstructionScript)

(fn QueueConstruction
  (params (Constructiion%20Struct :type Construction%20Struct%20Structure))
  (bind (_buildingclass _proxyclass _transform _displaymesh _buildtime) (Utilities|Struct|BreakConstruction_struct Constructiion%20Struct))
  (bind _returnvalue (Game|SpawnActorfromClass _proxyclass _transform "AlwaysSpawn" "MultiplyWithRoot" 0 _displaymesh 0))
  (CallFunction|BindConstruction _returnvalue)
  (Utilities|Array|Add (Variables|Default|GetProxies) _returnvalue)
  (Utilities|Array|Add (Variables|Default|Getqueue) Constructiion%20Struct)
  (Variables|/Game/Construction/ConstructionProxyBp.ConstructionProxyBp_C|SetConstructTime _returnvalue _buildtime))

(fn FinishConstruction
  (params (Proxy :type Construction%20Proxy%20Bp%20Object%20Reference))
  (bind _proxies (Variables|Default|GetProxies))
  (bind _queue (Variables|Default|Getqueue))
  (bind _output_get (LocalVariables|SetIndex (Utilities|Array|FindItem _proxies Proxy)))
  (LocalVariables|SetConfig (Utilities|Array|Get(acopy) _queue _output_get))
  (Utilities|Array|RemoveIndex _queue (LocalVariables|GetIndex))
  (Utilities|Array|RemoveIndex _proxies (LocalVariables|GetIndex))
  (Game|SpawnActorfromClass (.BuildingClass (Utilities|Struct|BreakConstruction_struct (LocalVariables|GetConfig))) (.Transform (Utilities|Struct|BreakConstruction_struct (LocalVariables|GetConfig))) "Undefined" "MultiplyWithRoot" 0 0 "NewEnumerator1" 0)
  (Actor|DestroyActor Proxy))